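; BP_FogBillboard is a placeable fog sheet that fakes fog with a flat mesh and a configurable material.
; Its Construction Script adds the mesh, scaled from the Size variable's X and Z, since depth is irrelevant on a flat sheet.
; It then creates a dynamic instance of FogSheetMasterMaterial and feeds it brightness-multiplied color, opacity, depth and distance fades, and panning noise settings.
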(fn `UserConstructionScript`
  (bind _fogsheetmid (`self.fogSheetMID`))
  (bind _brightness (`self.brightness`))
  (bind (_r _g _b _a) (`KismetMathLibrary.BreakColor` (`self.color`)))
  (bind _z (.z (* (`self.size`) 2.0)))
  (bind _returnvalue (`AddComponent|NODE_AddStaticMeshComponent-0` :`RelativeTransform` (`KismetMathLibrary.MakeTransform` (0.0 0.0 0.0) (struct) (`KismetMathLibrary.MakeVector` (.x (* (`self.size`) 2.0)) _z _z)))) ; Create fogsheet mesh
  (bind _returnvalue_2 (`PrimitiveComponent.CreateDynamicMaterialInstance` _returnvalue 0 (`self.FogSheetMasterMaterial`) "None"))
  (set `self.fogSheetMID` _returnvalue_2) ; Set the MID variable to apply settings to
  (`MaterialInstanceDynamic.SetVectorParameterValue` _fogsheetmid "Color" (`KismetMathLibrary.MakeColor` (* _r _brightness) (* _g _brightness) (* _b _brightness) _a))
  (`MaterialInstanceDynamic.SetScalarParameterValue` _fogsheetmid "MaxOpacity" (`self.opacity`))
  (`MaterialInstanceDynamic.SetScalarParameterValue` _fogsheetmid "DepthFadeDistance" (`self.depthFadeDistance`))
  (`MaterialInstanceDynamic.SetScalarParameterValue` _fogsheetmid "TilingMaskProjectionDistance" (`self.noiseProjectionDistance`))
  (`MaterialInstanceDynamic.SetScalarParameterValue` _fogsheetmid "NoiseSize" (`self.noiseSize`))
  (`MaterialInstanceDynamic.SetScalarParameterValue` _fogsheetmid "PanningSpeed" (`self.panningSpeed`))
  (`MaterialInstanceDynamic.SetScalarParameterValue` _fogsheetmid "FadeDistance" (`self.fadeDistance`)))